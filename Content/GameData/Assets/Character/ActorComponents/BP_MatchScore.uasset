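; BP_MatchScore is a character actor component for match scoring and records in a wrestling game.
; Its interface covers score display, time and objective scores, result type, team objectives, and match records for tags, eliminations, weapons, tables, explosions and thumbtacks.
; Tick functions are split into early-parameter, gameplay and match-result phases.
; All scoring functions here are empty or return defaults, and BeginPlay and Tick only call their parents.
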(fn `Add Objective`
  (params (Objective :type Byte)))

(fn `AddTeamObjective`
  (params (Objective :type Byte))
  (returns (Value :type Integer))
  (return 0))

(fn `AddTwoPlatoonCount`)

(fn `CalcTimeScore`
  (params (GameTime :type "Float (double-precision)") (MatchScore :type "/Game/GameData/Assets/Struct/MatchScore/FMatchScore_Main Structure"))
  (returns (TimeBase :type "Float (double-precision)") (TimeScore :type "Float (double-precision)"))
  (return 0.0 0.0))

(fn `GetDispScore`
  (params (DispMatchScoreParam :type "/Game/GameData/Assets/Struct/MatchScore/FDispMatchScoreParam Structure (by ref)") (WrestlerResultInfo :type "/Game/GameData/Assets/Struct/WrestlerResultInfo Structure")))

(fn `GetDispScore_Objective`
  (params (TargetMap :type "Map of Byte to Integer (by ref)"))
  (returns (ScoreObjective :type "Float (double-precision)") (ScoreAudience :type "Float (double-precision)"))
  (return 0.0 0.0))

(fn `GetDispScoreHP`
  (params (OwnerHP :type "Float (double-precision)"))
  (returns (HPRate :type "Float (double-precision)"))
  (return 0.0))

(fn `GetWrestlerResultType`
  (params (InGameInstance_I :type "/Game/GameData/Assets/GameInstance/BPI_ELGameInstance Interface") (MatchResultType :type Byte))
  (returns (WrestlerResultType :type "/Game/GameData/Assets/Enum/EWrestlerResultType Enum"))
  (return "NewEnumerator0"))

(fn `Match Records テーブルを破壊した`)

(fn `Match Records 凶器を当てた`
  (params (WeaponNo :type Integer)))

(fn `Match Records 凶器を被せた`)

(fn `Match Records 爆発を起こした`)

(fn `MatchRecords_タッチした`)

(fn `MatchRecords_バトルロイヤルで排除した`)

(fn `MatchRecords_画鋲に落とされた`)

(fn `MatchRecords_画鋲に落とした`)

(fn `ReceiveBeginPlay`
  (`parent.ReceiveBeginPlay`))

(fn `ReceiveTick`
  (params (DeltaSeconds :type "Float (double-precision)"))
  (`parent.ReceiveTick` DeltaSeconds))

(fn `Tick_EarlyParam`)

(fn `Tick_Gameplay`)

(fn `Tick_MatchResult`)